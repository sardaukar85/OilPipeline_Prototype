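; Procedural manager actor that builds a layout of Cube_Element actors from the DT_FirstPipeID data table.
; Reboot looks up each name in the RowName array and spawns a cube at that row's position and rotation, while Clear destroys all cubes.
; BeginPlay enables click events, and left click prints the actor under the cursor.
; Unconnected logic spawns cubes, cylinders and a spline-mesh BP_Arterya from TargetPoints.
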(event Custom|Reboot!
  (bind _row_name (Variables|Default|GetRow%20Name))
  (Utilities|FlowControl|Sequence
    (:then_4
      (for (_ _array_index) _row_name
        (bind _returnvalue (Utilities|GetDataTableRow "/Game/Alex3d/BP/DataTables/DT_FirstPipeID.DT_FirstPipeID" (Utilities|Array|Get(acopy) _row_name _array_index))
          (:then
            (Game|SpawnActorfromClass "/Game/Alex3d/BP/Elements/Cube_Element.Cube_Element_C" (Math|Transform|MakeTransform (Math|Vector|MakeVector (.f_x_position _returnvalue) (.f_y_position _returnvalue) (.f_z_position _returnvalue)) (Math|Rotator|MakeRotator (.f_roll_rotation _returnvalue) (.f_pitch_rotation _returnvalue) (.f_yaw_rotation _returnvalue)) "1.000000,1.000000,1.000000") "Undefined" "MultiplyWithRoot" 0 0)))))))

(event Custom|Clear!
  (bind _outactors (Actor|GetAllActorsOfClass "/Game/Alex3d/BP/Elements/Cube_Element.Cube_Element_C"))
  (for _array_element _outactors
    (Actor|DestroyActor _array_element)))

(event EventBeginPlay
  (Variables|/Script/Engine.PlayerController|SetbEnableClickEvents (Game|GetPlayerController 0) true))

(event Collision|EventActorBeginOverlap
  (params (OtherActor :type Actor%20Object%20Reference)))

(event EventTick
  (params (DeltaSeconds :type Float%20%28single-precision%29)))

(event Input|MouseEvents|DebugKeyLeftMouseButton
  (params (Key :type Key%20Structure :default "None") (ActionValue :type Input%20Action%20Value%20Structure)))

(event Input|MouseEvents|LeftMouseButton
  (params (Key :type Key%20Structure :default "None"))
  (:Pressed
    (Development|PrintString (Utilities|GetDisplayName (.HitActor (Collision|BreakHitResult (.HitResult (Game|Player|GetHitResultUnderCursorbyChannel (Game|GetPlayerController 0) "TraceTypeQuery1" true))))))))

(fn ConstructionScript)