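; BP_Rotator is an actor that turns a static mesh by RotationAngle and displays that angle as text.
; Its Rotation event first sets world yaw to the mesh's current roll plus RotationAngle, zeroing roll and pitch, then updates GradTXT.
; Because yaw builds on roll rather than current yaw, repeated calls do not accumulate rotation.
; Nothing in this Blueprint calls Rotation, and BeginPlay and Tick are disabled.
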(event Custom|Rotation
  (Utilities|FlowControl|Sequence
    (:then_0
      (Transformation|SetWorldRotation (Variables|Default|GetStaticMesh) (Math|Rotator|MakeRotator 0.0 0.0 (+ (.roll (Transformation|GetWorldRotation (Variables|Default|GetStaticMesh))) (Variables|Default|GetRotationAngle))) false false))
    (:then_1
      (Rendering|Components|TextRender|SetText (Variables|Default|GetGradTXT) (Utilities|Text|ToText(Float) (Variables|Default|GetRotationAngle) "HalfToEven")))))

(event EventBeginPlay)

(event Collision|EventActorBeginOverlap
  (params (OtherActor :type Actor%20Object%20Reference)))

(event EventTick
  (params (DeltaSeconds :type Float%20%28single-precision%29)))

(fn ConstructionScript)