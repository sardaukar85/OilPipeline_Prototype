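; BP_EasyManager is a manager actor for the BP_EasyElement pieces in the level.
; On BeginPlay it gathers every element, caches their types and world locations in separate arrays, then enables mouse click events on the player controller.
; A custom Go! event calls Click on the first gathered element, with no further logic acting on the cached data here.
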(event Custom|Go!
  (Default|Click (Utilities|Array|Get(acopy) (Variables|Default|GetElement_Array))))

(event EventBeginPlay
  (Utilities|FlowControl|Sequence
    (:then_0
      (bind _outactors (Actor|GetAllActorsOfClass "/Game/PipeProject/BP/Elements/BP_EasyElement.BP_EasyElement_C"))
      (bind _output_get (Variables|Default|SetElement_Array _outactors))
      (for _array_element _output_get
        (Utilities|Array|Add (Variables|Default|GetEasyElementsArray) (Utilities|Struct|MakeST_EasyElements (Variables|/Game/PipeProject/BP/Elements/BP_EasyElement.BP_EasyElement_C|GetElementType _array_element) 0.0 0.0))
        (Utilities|Array|Add (Variables|Default|GetElementLocationArray) (Math|Vector|MakeVector (.x (Transformation|GetActorLocation _array_element)) (.y (Transformation|GetActorLocation _array_element)) (.z (Transformation|GetActorLocation _array_element))))))
    (:then_1
      (Variables|/Script/Engine.PlayerController|SetbEnableClickEvents (Game|GetPlayerController 0) true))))

(event Collision|EventActorBeginOverlap
  (params (OtherActor :type Actor%20Object%20Reference)))

(event EventTick
  (params (DeltaSeconds :type Float%20%28single-precision%29)))

(fn ConstructionScript)