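; BP_ProceduralMeneger is the manager actor for pipe-element layouts, handling their spawning, indexing and clearing.
; On BeginPlay it records each Simple_Element's type and XY position, fires the ED Cell dispatcher, enables click events and spawns BP_Arterya at a TargetPoint.
; Reboot spawns element classes by Tag from DT_FirstPipeID rows, while Clear destroys all actors of listed classes.
; Click handlers print debug output, and position-range events are unfinished stubs.
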(event Custom|Reboot!
  (bind _row_name (Variables|Default|GetRow%20Name))
  (Utilities|FlowControl|Sequence
    (:then_4
      (for (_ _array_index) _row_name
        (bind _returnvalue (Utilities|GetDataTableRow "/Game/PipeProject/BP/DataTables/DT_FirstPipeID.DT_FirstPipeID" (Utilities|Array|Get(acopy) _row_name _array_index))
          (:then
            (switch name (.tag _returnvalue)
              (:Cube
                (Game|SpawnActorfromClass "/Game/PipeProject/BP/Elements/Cube_Element.Cube_Element_C" (Math|Transform|MakeTransform (Math|Vector|MakeVector (.f_x_position _returnvalue) (.f_y_position _returnvalue) (.f_z_position _returnvalue)) (Math|Rotator|MakeRotator (.f_roll_rotation _returnvalue) (.f_pitch_rotation _returnvalue) (.f_yaw_rotation _returnvalue)) "1.000000,1.000000,1.000000") "Undefined" "MultiplyWithRoot" 0 0))
              (:Cylinder
                (Game|SpawnActorfromClass "/Game/PipeProject/BP/Elements/Cylinder_Element.Cylinder_Element_C" (Math|Transform|MakeTransform (Math|Vector|MakeVector (.f_x_position _returnvalue) (.f_y_position _returnvalue) (.f_z_position _returnvalue)) (Math|Rotator|MakeRotator (.f_roll_rotation _returnvalue) (.f_pitch_rotation _returnvalue) (.f_yaw_rotation _returnvalue)) "1.000000,1.000000,1.000000") "Undefined" "MultiplyWithRoot" 0 0))
              (:Sphere
                (Game|SpawnActorfromClass "/Game/PipeProject/BP/Elements/Sphere_Element.Sphere_Element_C" (Math|Transform|MakeTransform (Math|Vector|MakeVector (.f_x_position _returnvalue) (.f_y_position _returnvalue) (.f_z_position _returnvalue)) (Math|Rotator|MakeRotator (.f_roll_rotation _returnvalue) (.f_pitch_rotation _returnvalue) (.f_yaw_rotation _returnvalue)) "1.000000,1.000000,1.000000") "Undefined" "MultiplyWithRoot" 0 0))
              (:Tube
                (Game|SpawnActorfromClass "/Game/PipeProject/BP/Elements/Tube_Element.Tube_Element_C" (Math|Transform|MakeTransform (Math|Vector|MakeVector (.f_x_position _returnvalue) (.f_y_position _returnvalue) (.f_z_position _returnvalue)) (Math|Rotator|MakeRotator (.f_roll_rotation _returnvalue) (.f_pitch_rotation _returnvalue) (.f_yaw_rotation _returnvalue)) "1.000000,1.000000,1.000000") "Undefined" "MultiplyWithRoot" 0 0))
              (:Cabel
                (Game|SpawnActorfromClass "/Game/PipeProject/BP/Elements/Cabel_Element.Cabel_Element_C" (Math|Transform|MakeTransform (Math|Vector|MakeVector (.f_x_position _returnvalue) (.f_y_position _returnvalue) (.f_z_position _returnvalue)) (Math|Rotator|MakeRotator (.f_roll_rotation _returnvalue) (.f_pitch_rotation _returnvalue) (.f_yaw_rotation _returnvalue)) "1.000000,1.000000,1.000000") "Undefined" "MultiplyWithRoot" 0 0)))))))))

(event Custom|Clear!
  (bind _actor_class (Variables|Default|GetActor%20Class))
  (bind _index (Utilities|FlowControl|ForLoopwithBreak 0 (Utilities|Array|Length _actor_class))
    (:LoopBody
      (bind _outactors (Actor|GetAllActorsOfClass (Utilities|Array|Get(acopy) _actor_class _index)))
      (for _array_element _outactors
        (Actor|DestroyActor _array_element)))))

(event Custom|ElementClick
  (Default|CallEDElement)
  (Development|PrintString "HI" true true "(R=0.000000,G=1.000000,B=0.054008,A=1.000000)"))

(event Custom|Cell_Reboot!
  (Utilities|FlowControl|Sequence
    (:then_0
      (bind _outactors (Actor|GetAllActorsOfClass "/Game/PipeProject/BP/Elements/Simple_Element.Simple_Element_C"))
      (for (_array_element _array_index) _outactors
        (Utilities|Array|SetArrayElem (Variables|Default|GetElements_X_Y) _array_index (Utilities|Struct|MakeST_Elements (Variables|/Game/PipeProject/BP/Elements/Simple_Element.Simple_Element_C|Gete_element_type _array_element) (Utilities|Struct|MakeST_XY (.x (Transformation|GetActorLocation _array_element)) (.y (Transformation|GetActorLocation _array_element)))))
        (Utilities|Array|Add (Variables|Default|GetPoint_Elements) (Variables|/Game/PipeProject/BP/Elements/Simple_Element.Simple_Element_C|Gete_element_type _array_element))))))

(event Custom|Elements_Reload!
  (bind _outactors (Actor|GetAllActorsOfClasswithTag "/Script/Engine.TargetPoint" "None"))
  (bind _returnvalue (Game|SpawnActorfromClass "/Game/Tram/Blueprints/BP_Arterya.BP_Arterya_C" (Transformation|GetActorTransform (Utilities|Array|Get(acopy) _outactors)) "Undefined" "MultiplyWithRoot" 0 0)))

(event Custom|Y-PointPosition
  (params (NewParam :type Float%20%28double-precision%29))
  (if (not (Math|Float|InRange(Float) NewParam 0.0 2.5e+02))
    (if (not (Math|Float|InRange(Float) NewParam 2.5e+02 5e+02))
      (if (not (Math|Float|InRange(Float) NewParam 5e+02 7.5e+02))
        (if (Math|Float|InRange(Float) NewParam 7.5e+02 1e+03)
          _)))))

(event Custom|XY-PointPosition
  (params (X :type Float%20%28double-precision%29) (Y :type Float%20%28double-precision%29))
  (Utilities|FlowControl|Sequence
    (:then_0
      (if (not (Math|Float|InRange(Float) X 0.0 1e+02))
        (if (not (>= X 0.0))
          (if (not (>= X 25.0))
            (if (not (>= X 5e+01))
              (if (>= X 75.0)
                _))))))))

(event EventBeginPlay
  (Utilities|FlowControl|Sequence
    (:then_0
      (CallFunction|CellReboot!) ; обновляем все ячейки и типы элементов
    )
    (:then_1
      (Default|CallEDCell))
    (:then_2
      (Variables|/Script/Engine.PlayerController|SetbEnableClickEvents (Game|GetPlayerController 0) true))
    (:then_4
      (CallFunction|ElementsReload!))))

(event Collision|EventActorBeginOverlap
  (params (OtherActor :type Actor%20Object%20Reference)))

(event EventTick
  (params (DeltaSeconds :type Float%20%28single-precision%29)))

(event Input|MouseEvents|DebugKeyLeftMouseButton
  (params (Key :type Key%20Structure :default "None") (ActionValue :type Input%20Action%20Value%20Structure)))

(event Input|MouseEvents|LeftMouseButton
  (params (Key :type Key%20Structure :default "None"))
  (:Pressed
    (Development|PrintString (Utilities|GetDisplayName (.HitActor (Collision|BreakHitResult (.HitResult (Game|Player|GetHitResultUnderCursorbyChannel (Game|GetPlayerController 0) "TraceTypeQuery1" true))))))))

(fn ConstructionScript)