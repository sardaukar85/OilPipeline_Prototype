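; BP_Clapan is a clickable valve element in the pipe project that links its mesh to a matching UI element.
; Pressing the mesh applies a green outline overlay material, and releasing clears it.
; Both actions reach UI_TestOil through BP_ProceduralMeneger and use PIDIndex to turn one of three button backgrounds red or back to transparent.
; Rotation and Invisible events are empty stubs.
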(event OnClicked(Mesh)
  (params (TouchedComponent :type Primitive%20Component%20Object%20Reference) (ButtonPressed :type Key%20Structure :default "None"))
  (CallFunction|Outline!)
  (bind _asbp_procedural_meneger (Utilities|Casting|CastToBP_ProceduralMeneger (Variables|Default|GetProceduralManagerRef)))
  (bind _asui_test_oil (Utilities|Casting|CastToUI_TestOil (Variables|/Game/PipeProject/BP/CoreGameplay/BP_ProceduralMeneger.BP_ProceduralMeneger_C|GetUI_Ref _asbp_procedural_meneger)))
  (switch int (Variables|Default|GetP&ID_Index)
    (:0
      (Variables|/Script/UMG.Button|SetBackgroundColor (Variables|/Game/PipeProject/UI/UI_TestOil.UI_TestOil_C|GetButton_Element1 _asui_test_oil) "(R=0.994792,G=0.000000,B=0.000000,A=1.000000)"))
    (:1
      (Variables|/Script/UMG.Button|SetBackgroundColor (Variables|/Game/PipeProject/UI/UI_TestOil.UI_TestOil_C|GetButton_Element2 _asui_test_oil) "(R=1.000000,G=0.000000,B=0.000000,A=1.000000)"))
    (:2
      (Variables|/Script/UMG.Button|SetBackgroundColor (Variables|/Game/PipeProject/UI/UI_TestOil.UI_TestOil_C|GetButton_Element3 _asui_test_oil) "(R=1.000000,G=0.000000,B=0.000000,A=1.000000)"))))

(event OnReleased(Mesh)
  (params (TouchedComponent :type Primitive%20Component%20Object%20Reference) (ButtonReleased :type Key%20Structure :default "None"))
  (CallFunction|OutlineOff!)
  (bind _asbp_procedural_meneger (Utilities|Casting|CastToBP_ProceduralMeneger (Variables|Default|GetProceduralManagerRef)))
  (bind _asui_test_oil (Utilities|Casting|CastToUI_TestOil (Variables|/Game/PipeProject/BP/CoreGameplay/BP_ProceduralMeneger.BP_ProceduralMeneger_C|GetUI_Ref _asbp_procedural_meneger)))
  (switch int (Variables|Default|GetP&ID_Index)
    (:0
      (Variables|/Script/UMG.Button|SetBackgroundColor (Variables|/Game/PipeProject/UI/UI_TestOil.UI_TestOil_C|GetButton_Element1 _asui_test_oil) "(R=0.994792,G=0.994792,B=0.994792,A=0.000000)"))
    (:1
      (Variables|/Script/UMG.Button|SetBackgroundColor (Variables|/Game/PipeProject/UI/UI_TestOil.UI_TestOil_C|GetButton_Element2 _asui_test_oil) "(R=1.000000,G=1.000000,B=1.000000,A=0.000000)"))
    (:2
      (Variables|/Script/UMG.Button|SetBackgroundColor (Variables|/Game/PipeProject/UI/UI_TestOil.UI_TestOil_C|GetButton_Element3 _asui_test_oil) "(R=1.000000,G=1.000000,B=1.000000,A=0.000000)"))))

(event Custom|Rotation!)

(event Custom|Outline!
  (Rendering|Material|SetOverlayMaterial (Variables|Default|GetMesh) "/Game/Tram/MTL/Outline/MI_Outline_Green.MI_Outline_Green" :!class /Script/Engine.MeshComponent) ; Оутлайнер ВКЛ
  (Variables|Default|SetIsOutlineWork? true))

(event Custom|Invisible!)

(event Custom|OutlineOff!
  (Rendering|Material|SetOverlayMaterial (Variables|Default|GetMesh) 0 :!class /Script/Engine.MeshComponent) ; Оутлайнер ВКЛ
  (Variables|Default|SetIsOutlineWork? false))

(event EventBeginPlay)

(event Collision|EventActorBeginOverlap
  (params (OtherActor :type Actor%20Object%20Reference)))

(event EventTick
  (params (DeltaSeconds :type Float%20%28single-precision%29)))

(fn ConstructionScript)