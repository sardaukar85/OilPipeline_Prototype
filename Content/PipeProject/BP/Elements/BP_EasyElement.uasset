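; BP_EasyElement is a clickable pipe-system element, such as a tube, valve, gauge, lever or toggle.
; The construction script picks mesh and material by element type, finds BP_EasyManager, and attaches a cable to TubeEnd or hides it on end pieces.
; Clicking applies a random overlay material as a temporary outline.
; It also briefly shows a UI_TXT_Message widget at the cursor, with text selected by PoitIndex.
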(event OnClicked(Mesh)
  (params (TouchedComponent :type Primitive%20Component%20Object%20Reference) (ButtonPressed :type Key%20Structure :default "None"))
  (Utilities|FlowControl|Sequence
    (:then_0
      (CallFunction|Click))
    (:then_1
      (bind _returnvalue (Class|WidgetLayoutLibrary|GetMousePositiononViewport))
      (bind _returnvalue_2 (UserInterface|CreateWidget "/Game/PipeProject/UI/UI_TXT_Message.UI_TXT_Message_C"))
      (UserInterface|Viewport|AddtoViewport _returnvalue_2 0)
      (Variables|/Game/PipeProject/UI/UI_TXT_Message.UI_TXT_Message_C|SetTXT%20Message _returnvalue_2 (Utilities|Array|Get(acopy) (Variables|/Game/PipeProject/UI/UI_TXT_Message.UI_TXT_Message_C|GetMessageTXT _returnvalue_2) (Variables|Default|GetPoit_Index)))
      (Class|Widget|SetRenderTransform _returnvalue_2 (Utilities|Struct|MakeWidgetTransform _returnvalue "(X=1.000000,Y=1.000000)" "(X=0.000000,Y=0.000000)" 0.0))
      (Utilities|FlowControl|Delay 2.0)
      (Widget|RemovefromParent _returnvalue_2))))

(event EDEasy(ManagerRef))

(event OnBeginCursorOver(Mesh)
  (params (TouchedComponent :type Primitive%20Component%20Object%20Reference)))

(event OnEndCursorOver(Mesh)
  (params (TouchedComponent :type Primitive%20Component%20Object%20Reference)))

(event Custom|Click
  (bind _mesh (Variables|Default|GetMesh))
  (Rendering|Material|SetOverlayMaterial _mesh (Utilities|Array|Get(acopy) (Variables|Default|GetNew%20Overlay%20Material) (Math|Random|RandomInteger 3)) :!class /Script/Engine.MeshComponent) ; Оутлайнер ВКЛ
  (Utilities|FlowControl|Delay 3.0)
  (Rendering|Material|SetOverlayMaterial _mesh 0 :!class /Script/Engine.MeshComponent) ; Оутлайнер ВКЛ
)

(event EventBeginPlay)

(event Collision|EventActorBeginOverlap
  (params (OtherActor :type Actor%20Object%20Reference)))

(event EventTick
  (params (DeltaSeconds :type Float%20%28single-precision%29)))

(fn ConstructionScript
  (bind _mesh (Variables|Default|GetMesh))
  (Utilities|FlowControl|Sequence
    (:then_0
      (switch Utilities|FlowControl|Switch|SwitchonE_ElementsType (Variables|Default|GetElementType)
        (:NewEnumerator6
          (Variables|Default|SetElement%20Index 0))
        (:NewEnumerator0
          (Variables|Default|SetElement%20Index 1))
        (:NewEnumerator1
          (Variables|Default|SetElement%20Index 2))
        (:NewEnumerator2
          (Variables|Default|SetElement%20Index 3))
        (:NewEnumerator3
          (Variables|Default|SetElement%20Index 4))
        (:NewEnumerator4
          (Variables|Default|SetElement%20Index 5))
        (:NewEnumerator5
          (Variables|Default|SetElement%20Index 6))))
    (:then_1
      (if (Variables|Default|GetIsTubeEnd?)
        (Rendering|SetVisibility (Variables|Default|GetCable) false false)
        (else
          (Class|CableComponent|SetAttachEndto (Variables|Default|GetCable) (Variables|Default|GetTubeEnd) "None" "None"))))
    (:then_2
      (Components|StaticMesh|SetStaticMesh _mesh (Utilities|Array|Get(acopy) (Variables|Default|GetMeshRef) (Variables|Default|GetElement%20Index)))
      (Rendering|Material|SetMaterial _mesh 0 (Utilities|Array|Get(acopy) (Variables|Default|GetMaterialRef) (Variables|Default|GetElement%20Index))))
    (:then_3
      (bind _outactors (Actor|GetAllActorsOfClass "/Game/PipeProject/BP/CoreGameplay/BP_EasyManager.BP_EasyManager_C"))
      (Variables|Default|SetManagerRef (Utilities|Array|Get(acopy) _outactors)))))