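; Clickable pipe-project element that links its mesh to a button in the UI_TestOil widget through PIDIndex.
; On click it applies a green overlay outline, tints the indexed button, calls the widget's Hello, then passes its PID to BP_ProceduralMeneger and calls ElementClick.
; On release it clears the outline and resets only the first three buttons, using indices offset from the click mapping.
; Rotation and Invisible are empty stubs.
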(event OnClicked(Mesh)
  (params (TouchedComponent :type Primitive%20Component%20Object%20Reference) (ButtonPressed :type Key%20Structure :default "None"))
  (Utilities|FlowControl|Sequence
    (:then_0
      (CallFunction|Outline!)
      (Development|PrintString "Hello"))
    (:then_1
      (bind _asui_test_oil (Utilities|Casting|CastToUI_TestOil (Variables|Default|GetUITestOilRef)))
      (switch int (Variables|Default|GetP&ID_Index)
        (:1
          (Variables|/Script/UMG.Button|SetBackgroundColor (Variables|/Game/PipeProject/UI/UI_TestOil.UI_TestOil_C|GetButton_Element1 _asui_test_oil) "(R=0.994792,G=0.000000,B=0.000000,A=1.000000)")
          (Utilities|FlowControl|Delay 3.0))
        (:2
          (Variables|/Script/UMG.Button|SetBackgroundColor (Variables|/Game/PipeProject/UI/UI_TestOil.UI_TestOil_C|GetButton_Element2 _asui_test_oil) "(R=1.000000,G=0.000000,B=0.000000,A=1.000000)"))
        (:3
          (Variables|/Script/UMG.Button|SetBackgroundColor (Variables|/Game/PipeProject/UI/UI_TestOil.UI_TestOil_C|GetButton_Element3 _asui_test_oil) "(R=1.000000,G=0.000000,B=0.000000,A=1.000000)"))
        (:4
          (Variables|/Script/UMG.Button|SetBackgroundColor (Variables|/Game/PipeProject/UI/UI_TestOil.UI_TestOil_C|GetButton_Element4 _asui_test_oil) "(R=1.000000,G=0.000000,B=0.000000,A=1.000000)"))
        (:5
          (Variables|/Script/UMG.Button|SetBackgroundColor (Variables|/Game/PipeProject/UI/UI_TestOil.UI_TestOil_C|GetButton_Element5 _asui_test_oil) "(R=1.000000,G=0.000000,B=0.000000,A=1.000000)"))
        (:6
          (Variables|/Script/UMG.Button|SetBackgroundColor (Variables|/Game/PipeProject/UI/UI_TestOil.UI_TestOil_C|GetButton_Element6 _asui_test_oil) "(R=1.000000,G=0.000000,B=0.000000,A=1.000000)"))
        (:7
          (Variables|/Script/UMG.Button|SetBackgroundColor (Variables|/Game/PipeProject/UI/UI_TestOil.UI_TestOil_C|GetButton_Element7 _asui_test_oil) "(R=0.337497,G=0.774423,B=1.000000,A=0.100000)"))
        (:8
          (Variables|/Script/UMG.Button|SetBackgroundColor (Variables|/Game/PipeProject/UI/UI_TestOil.UI_TestOil_C|GetButton_Element8 _asui_test_oil) "(R=1.000000,G=0.000000,B=0.000000,A=1.000000)"))
        (:9
          (Variables|/Script/UMG.Button|SetBackgroundColor (Variables|/Game/PipeProject/UI/UI_TestOil.UI_TestOil_C|GetButton_Element9 _asui_test_oil) "(R=0.000000,G=1.000000,B=0.474488,A=0.500000)"))
        (:10
          (Variables|/Script/UMG.Button|SetBackgroundColor (Variables|/Game/PipeProject/UI/UI_TestOil.UI_TestOil_C|GetButton_Element10 _asui_test_oil) "(R=1.000000,G=0.306013,B=0.963941,A=0.500000)"))
        (:11
          (Variables|/Script/UMG.Button|SetBackgroundColor (Variables|/Game/PipeProject/UI/UI_TestOil.UI_TestOil_C|GetButton_Element11 _asui_test_oil) "(R=1.000000,G=0.100239,B=0.957907,A=0.500000)"))
        (:12
          (Variables|/Script/UMG.Button|SetBackgroundColor (Variables|/Game/PipeProject/UI/UI_TestOil.UI_TestOil_C|GetButton_Element12 _asui_test_oil) "(R=1.000000,G=0.000000,B=0.000000,A=1.000000)"))
        (:13
          (Variables|/Script/UMG.Button|SetBackgroundColor (Variables|/Game/PipeProject/UI/UI_TestOil.UI_TestOil_C|GetButton_Element13 _asui_test_oil) "(R=1.000000,G=0.000000,B=0.000000,A=1.000000)"))
        (:14
          (Variables|/Script/UMG.Button|SetBackgroundColor (Variables|/Game/PipeProject/UI/UI_TestOil.UI_TestOil_C|GetButton_Element14 _asui_test_oil) "(R=1.000000,G=0.000000,B=0.000000,A=1.000000)"))
        (:15
          (Variables|/Script/UMG.Button|SetBackgroundColor (Variables|/Game/PipeProject/UI/UI_TestOil.UI_TestOil_C|GetButton_Element14 _asui_test_oil) "(R=1.000000,G=0.000000,B=0.000000,A=1.000000)"))
        (:16
          (Variables|/Script/UMG.Button|SetBackgroundColor (Variables|/Game/PipeProject/UI/UI_TestOil.UI_TestOil_C|GetButton_Element15 _asui_test_oil) "(R=1.000000,G=0.000000,B=0.000000,A=1.000000)"))
        (:17
          (Variables|/Script/UMG.Button|SetBackgroundColor (Variables|/Game/PipeProject/UI/UI_TestOil.UI_TestOil_C|GetButton_Element16 _asui_test_oil) "(R=1.000000,G=0.000000,B=0.000000,A=1.000000)"))
        (:18
          (Variables|/Script/UMG.Button|SetBackgroundColor (Variables|/Game/PipeProject/UI/UI_TestOil.UI_TestOil_C|GetButton_Element17 _asui_test_oil) "(R=1.000000,G=0.000000,B=0.000000,A=1.000000)"))
        (:19
          (Variables|/Script/UMG.Button|SetBackgroundColor (Variables|/Game/PipeProject/UI/UI_TestOil.UI_TestOil_C|GetButton_Element18 _asui_test_oil) "(R=1.000000,G=0.000000,B=0.000000,A=1.000000)"))
        (:20
          (Variables|/Script/UMG.Button|SetBackgroundColor (Variables|/Game/PipeProject/UI/UI_TestOil.UI_TestOil_C|GetButton_Element20 _asui_test_oil) "(R=1.000000,G=0.000000,B=0.000000,A=1.000000)"))
        (:21
          (Variables|/Script/UMG.Button|SetBackgroundColor (Variables|/Game/PipeProject/UI/UI_TestOil.UI_TestOil_C|GetButton_Element21 _asui_test_oil) "(R=1.000000,G=0.000000,B=0.000000,A=1.000000)"))
        (:22
          (Variables|/Script/UMG.Button|SetBackgroundColor (Variables|/Game/PipeProject/UI/UI_TestOil.UI_TestOil_C|GetButton_Element22 _asui_test_oil) "(R=1.000000,G=0.000000,B=0.000000,A=1.000000)"))))
    (:then_2
      (bind _asui_test_oil_2 (Utilities|Casting|CastToUI_TestOil (Variables|Default|GetUITestOilRef)))
      (Default|Hello! _asui_test_oil_2))
    (:then_3
      (bind _asbp_procedural_meneger (Utilities|Casting|CastToBP_ProceduralMeneger (Variables|Default|GetProceduralManagerRef)))
      (Variables|/Game/PipeProject/BP/CoreGameplay/BP_ProceduralMeneger.BP_ProceduralMeneger_C|SetP&ID _asbp_procedural_meneger (Variables|Default|GetP&ID_Index))
      (Default|ElementClick _asbp_procedural_meneger))))

(event OnReleased(Mesh)
  (params (TouchedComponent :type Primitive%20Component%20Object%20Reference) (ButtonReleased :type Key%20Structure :default "None"))
  (CallFunction|OutlineOff!)
  (bind _asbp_procedural_meneger (Utilities|Casting|CastToBP_ProceduralMeneger (Variables|Default|GetProceduralManagerRef)))
  (bind _asui_test_oil (Utilities|Casting|CastToUI_TestOil (Variables|/Game/PipeProject/BP/CoreGameplay/BP_ProceduralMeneger.BP_ProceduralMeneger_C|GetUI_Ref _asbp_procedural_meneger)))
  (switch int (Variables|Default|GetP&ID_Index)
    (:0
      (Variables|/Script/UMG.Button|SetBackgroundColor (Variables|/Game/PipeProject/UI/UI_TestOil.UI_TestOil_C|GetButton_Element1 _asui_test_oil) "(R=0.994792,G=0.994792,B=0.994792,A=0.000000)"))
    (:1
      (Variables|/Script/UMG.Button|SetBackgroundColor (Variables|/Game/PipeProject/UI/UI_TestOil.UI_TestOil_C|GetButton_Element2 _asui_test_oil) "(R=1.000000,G=1.000000,B=1.000000,A=0.000000)"))
    (:2
      (Variables|/Script/UMG.Button|SetBackgroundColor (Variables|/Game/PipeProject/UI/UI_TestOil.UI_TestOil_C|GetButton_Element3 _asui_test_oil) "(R=1.000000,G=1.000000,B=1.000000,A=0.000000)"))))

(event Custom|Rotation!)

(event Custom|Outline!
  (Rendering|Material|SetOverlayMaterial (Variables|Default|GetMesh) "/Game/Tram/MTL/Outline/MI_Outline_Green.MI_Outline_Green" :!class /Script/Engine.MeshComponent) ; Оутлайнер ВКЛ
  (Variables|Default|SetIsOutlineWork? true))

(event Custom|Invisible!)

(event Custom|OutlineOff!
  (Rendering|Material|SetOverlayMaterial (Variables|Default|GetMesh) 0 :!class /Script/Engine.MeshComponent) ; Оутлайнер ВКЛ
  (Variables|Default|SetIsOutlineWork? false))

(event EventBeginPlay
  (Utilities|Casting|CastToBP_ProceduralMeneger (Variables|Default|GetProceduralManagerRef)))

(event Collision|EventActorBeginOverlap
  (params (OtherActor :type Actor%20Object%20Reference)))

(event EventTick
  (params (DeltaSeconds :type Float%20%28single-precision%29)))

(fn ConstructionScript)