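; Pipe element actor that can display one of several meshes from ElementsLibrary, such as tube, valve, gauge, meter, lever or toggle.
; The ElementUpdate event sets the Mesh component to the library entry at MeshIndex.
; Switches mapping EElementType to MeshIndex sit disconnected in both the event graph and construction script, so MeshIndex is not derived from the type here.
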(event Custom|ElementUpdate!
  (Components|StaticMesh|SetStaticMesh (Variables|Default|GetMesh) (Utilities|Array|Get(acopy) (Variables|Default|GetElements_Library) (Variables|Default|GetMesh_Index))))

(event EventBeginPlay)

(event Collision|EventActorBeginOverlap
  (params (OtherActor :type Actor%20Object%20Reference)))

(event EventTick
  (params (DeltaSeconds :type Float%20%28single-precision%29)))

(fn ConstructionScript)