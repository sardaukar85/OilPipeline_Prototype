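; BP_Vector_Variable is an actor that displays the world location of its Sphere component as X, Y and Z text values.
; On BeginPlay it starts a looping half-second timer bound to a custom event, so the readout refreshes without using Tick.
; Each timer call reads the Sphere's world location and writes each axis, converted to text, into TXTX, TXTY and TXTZ.
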(event Custom|CustomEvent
  (bind _sphere (Variables|Default|GetSphere))
  (bind _returnvalue (Transformation|GetWorldLocation _sphere))
  (Rendering|Components|TextRender|SetText (Variables|Default|GetTXT_X) (Utilities|Text|ToText(Float) (.x _returnvalue) "HalfToEven"))
  (Rendering|Components|TextRender|SetText (Variables|Default|GetTXT_Y) (Utilities|Text|ToText(Float) (.y _returnvalue) "HalfToEven"))
  (Rendering|Components|TextRender|SetText (Variables|Default|GetTXT_Z) (Utilities|Text|ToText(Float) (.z _returnvalue) "HalfToEven")))

(event EventBeginPlay
  (Utilities|Time|SetTimerbyEvent (delegate Custom|CustomEvent) 0.5 true))

(event Collision|EventActorBeginOverlap
  (params (OtherActor :type Actor%20Object%20Reference)))

(event EventTick
  (params (DeltaSeconds :type Float%20%28single-precision%29)))

(fn ConstructionScript)